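; BP_AICharacter is an AI character that randomizes its appearance and changes movement speed with its target state.
; On BeginPlay it randomly picks the male or female mannequin skeletal mesh.
; FindTarget and LostTarget events switch CharacterMovement between a faster speed while a target is found and a slower one when it is lost.
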(event `self.ReceiveBeginPlay`
  ;[1 1 1] 성별 랜덤 설정
  (`SkinnedMeshComponent.SetSkinnedAssetAndUpdate` (`self.Mesh`) (select `bool` (`KismetMathLibrary.RandomBool`) :`false` "/Game/Meshes/Mannequin/Character/Mesh/SK_Mannequin_Female.SK_Mannequin_Female" :`true` "/Game/Meshes/Mannequin/Character/Mesh/SK_Mannequin.SK_Mannequin" :!type "SkeletalMesh Object Reference") true))

(event `/Game/Blueprints/AI/IBP_AI.LostTarget`
  (params (TargetInfo :type "ActorPerceptionUpdateInfo Structure"))
  (set `CharacterMovementComponent.MaxWalkSpeed` 200.0 (`self.CharacterMovement`)))

(event `/Game/Blueprints/AI/IBP_AI.FindTarget`
  (params (TargetInfo :type "ActorPerceptionUpdateInfo Structure"))
  (set `CharacterMovementComponent.MaxWalkSpeed` 500.0 (`self.CharacterMovement`)))

(fn `UserConstructionScript`
  (`parent.UserConstructionScript`))